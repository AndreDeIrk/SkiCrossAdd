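; Physics ball actor that launches along its forward vector at a set speed and destroys itself after its lifetime.
; On spawn it joins the background layer, and its construction script gives the mesh a random rotation.
; Each tick it adds wind to its velocity, scaled by delta time and the strength of the first BP_BallWind found in the level.
; Layer-crossing and constant-speed logic are present but disconnected.
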(event EventBeginPlay
  (Class|LayersBlueprintLibrary|AddActortoLayer self (Variables|Default|GetBGLayer))
  (Utilities|FlowControl|Sequence
    (:then_0
      (Utilities|FlowControl|Delay (Variables|Settings|GetLifeTime))
      (Actor|DestroyActor))
    (:then_1
      (Physics|SetPhysicsLinearVelocity (Variables|Default|GetStaticMesh) (* (Transformation|GetActorForwardVector) (Variables|Settings|GetSpeed)) false "None"))))

(event EventTick
  (params (DeltaSeconds :type Float%20%28single-precision%29))
  (Utilities|FlowControl|Sequence
    (:then_0
      (bind _outactors (Actor|GetAllActorsOfClass "/Game/Blueprints/BallsEmitter/BP_BallWind.BP_BallWind_C"))
      (bind _returnvalue (Physics|GetPhysicsLinearVelocity (Variables|Default|GetStaticMesh) "None"))
      (Physics|SetPhysicsLinearVelocity (Variables|Default|GetStaticMesh) (+ _returnvalue (* (Variables|Default|GetWind) (Variables|/Game/Blueprints/BallsEmitter/BP_BallWind.BP_BallWind_C|GetWindStrength (Utilities|Array|Get(acopy) _outactors)) (Utilities|Time|GetWorldDeltaSeconds))) false "None"))))

(fn ConstructionScript
  (Transformation|SetRelativeRotation (Variables|Default|GetStaticMesh) (Math|Random|RandomRotator true) false false))