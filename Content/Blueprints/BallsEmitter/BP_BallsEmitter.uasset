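; BP_BallsEmitter is an actor that spawns a timed series of BP_Ball actors at random points inside its Box component.
; ProvideBallsSpawning loops through a Delay until BallsNumber is reached, then resets its counter; BeginPlay is empty and nothing connected here triggers it.
; SpawnBall passes lifetime, speed and normalized wind to each scaled-down ball, aligns it to the box's rotation and adds it to ObjectsLayer.
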(event Custom|ProvideBallsSpawning
  (if (> (Variables|Default|GetBallsNumber) (Variables|Default|GetCounter)) :!label _label
    (CallFunction|SpawnBall)
    (Utilities|FlowControl|Delay (Variables|Settings|GetSpawnInterval))
    (Math|Integer|IncrementInt (Variables|Default|GetCounter)
      (:%20%20
        (Development|PrintString (Utilities|String|ToString(Integer) (Variables|Default|GetCounter)))
        (goto _label)))
    (else
      (Variables|Default|SetCounter 0))))

(event EventBeginPlay)

(fn ConstructionScript)

(fn SpawnBall
  (bind _returnvalue (Game|SpawnActorfromClass "/Game/Blueprints/BallsEmitter/BP_Ball.BP_Ball_C" (Math|Transform|MakeTransform (CallFunction|GetSpawnLocation) (Transformation|GetWorldRotation (Variables|Default|GetBox)) "0.700000,0.700000,0.700000") "Undefined" 0 (Variables|Settings|GetBallsLifeTime) (Variables|Settings|GetBallsSpeed) 0))
  (Class|LayersBlueprintLibrary|AddActortoLayer _returnvalue (Variables|Default|GetObjectsLayer))
  (Variables|/Game/Blueprints/BallsEmitter/BP_Ball.BP_Ball_C|SetWind _returnvalue (Math|Vector|Normalize (Variables|Default|GetWind))))

(fn GetSpawnLocation
  (bind _box (Variables|Default|GetBox))
  (bind _returnvalue (Components|Box|GetScaledBoxExtent _box))
  (return (+ (Transformation|GetWorldLocation (Variables|Default|GetBox)) (Math|Vector|MakeVector (* (Math|Random|RandomFloatinRange -1.0 1.0) (.x _returnvalue)) (* (Math|Random|RandomFloatinRange -1.0 1.0) (.y _returnvalue)) (* (Math|Random|RandomFloatinRange -1.0 1.0) (.z _returnvalue))))))