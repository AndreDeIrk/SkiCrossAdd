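; Animated SENTRO GROUP logo actor, hidden at BeginPlay, that plays a timed reveal and exit when Appearing is called.
; Staggered timelines scale and move the Ball and spin-scale each letter in, with the last also driving the Ball's VisibilityPercent material parameter.
; After a hold, Disappearing reverses the letter timelines in the same order and shrinks the Ball.
; CommandsReceivingAvailable blocks retriggering until then; the Niagara VFX nodes are unconnected.
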(event Custom|Appearing
  (Rendering|SetActorHiddenInGame false)
  (if (Variables|Properties|GetCommandsReceivingAvailable)
    (CallFunction|SetCommandsReceiving false)
    (CallFunction|ResetState)
    (Default|CallAnimationStarted)
    (Utilities|FlowControl|Sequence
      (:then_0
        (Utilities|FlowControl|Delay 0.2))
      (:then_1
        (Utilities|FlowControl|Sequence
          (:then_0
            (Utilities|FlowControl|Sequence
              (:then_0
                (Utilities|FlowControl|Sequence
                  (:then_0
                    (bind _value (Timeline|BallScaling PlayFromStart)
                      (:Update
                        (Transformation|SetRelativeScale3D (Variables|Default|GetBall) (Math|Vector|Lerp(Vector) "0, 0, 0" "0.730000,0.730000,0.730000" _value)))))
                  (:then_1
                    (Utilities|FlowControl|Delay 0.32)
                    (bind _value_2 (Timeline|BallMoving PlayFromStart)
                      (:Update
                        (Transformation|SetRelativeLocation (Variables|Default|GetBall) (Math|Vector|Lerp(Vector) "0, 0, 0" "151.419613,0.000000,3.531468" _value_2) false false))))))
              (:then_1
                (Utilities|FlowControl|Delay 0.2)
                (bind _value_3 (Timeline|SRotation PlayFromStart)
                  (:Update
                    (Transformation|SetRelativeRotation (Variables|Default|GetS) (Math|Rotator|Lerp(Rotator) "180.000000,0.000000,0.000000" "0, 0, 0" _value_3) false false)
                    (Transformation|SetRelativeScale3D (Variables|Default|GetS) (Math|Vector|Lerp(Vector) "0, 0, 0" "1.000000,1.000000,1.000000" _value_3)))))
              (:then_2
                (Utilities|FlowControl|Delay 0.44)
                (bind _value_4 (Timeline|ERotation PlayFromStart)
                  (:Update
                    (Transformation|SetRelativeRotation (Variables|Default|GetE) (Math|Rotator|Lerp(Rotator) "180.000000,0.000000,0.000000" "0, 0, 0" _value_4) false false)
                    (Transformation|SetRelativeScale3D (Variables|Default|GetE) (Math|Vector|Lerp(Vector) "0, 0, 0" "1.000000,1.000000,1.000000" _value_4)))))
              (:then_3
                (Utilities|FlowControl|Delay 0.56)
                (bind _value_5 (Timeline|NRotation PlayFromStart)
                  (:Update
                    (Transformation|SetRelativeRotation (Variables|Default|GetN) (Math|Rotator|Lerp(Rotator) "180.000000,0.000000,0.000000" "0, 0, 0" _value_5) false false)
                    (Transformation|SetRelativeScale3D (Variables|Default|GetN) (Math|Vector|Lerp(Vector) "0, 0, 0" "1.000000,1.000000,1.000000" _value_5)))))
              (:then_4
                (Utilities|FlowControl|Delay 0.68)
                (bind _value_6 (Timeline|TRotation PlayFromStart)
                  (:Update
                    (Transformation|SetRelativeRotation (Variables|Default|GetT) (Math|Rotator|Lerp(Rotator) "180.000000,0.000000,0.000000" "0, 0, 0" _value_6) false false)
                    (Transformation|SetRelativeScale3D (Variables|Default|GetT) (Math|Vector|Lerp(Vector) "0, 0, 0" "1.000000,1.000000,1.000000" _value_6)))))
              (:then_5
                (Utilities|FlowControl|Delay 0.8)
                (bind _value_7 (Timeline|R1Rotation PlayFromStart)
                  (:Update
                    (Transformation|SetRelativeRotation (Variables|Default|GetR1) (Math|Rotator|Lerp(Rotator) "180.000000,0.000000,0.000000" "0, 0, 0" _value_7) false false)
                    (Transformation|SetRelativeScale3D (Variables|Default|GetR1) (Math|Vector|Lerp(Vector) "0, 0, 0" "1.000000,1.000000,1.000000" _value_7)))))))
          (:then_1
            (Utilities|FlowControl|Sequence
              (:then_0
                (Utilities|FlowControl|Delay 0.68)
                (bind _value_8 (Timeline|GRotation PlayFromStart)
                  (:Update
                    (Transformation|SetRelativeRotation (Variables|Default|GetG) (Math|Rotator|Lerp(Rotator) "180.000000,0.000000,0.000000" "0, 0, 0" _value_8) false false)
                    (Transformation|SetRelativeScale3D (Variables|Default|GetG) (Math|Vector|Lerp(Vector) "0, 0, 0" "1.000000,1.000000,1.000000" _value_8)))))
              (:then_1
                (Utilities|FlowControl|Delay 0.84)
                (bind _value_9 (Timeline|R2Rotation PlayFromStart)
                  (:Update
                    (Transformation|SetRelativeRotation (Variables|Default|GetR2) (Math|Rotator|Lerp(Rotator) "180.000000,0.000000,0.000000" "0, 0, 0" _value_9) false false)
                    (Transformation|SetRelativeScale3D (Variables|Default|GetR2) (Math|Vector|Lerp(Vector) "0, 0, 0" "1.000000,1.000000,1.000000" _value_9)))))
              (:then_2
                (Utilities|FlowControl|Delay 0.92)
                (bind _value_10 (Timeline|ORotation PlayFromStart)
                  (:Update
                    (Transformation|SetRelativeRotation (Variables|Default|GetO) (Math|Rotator|Lerp(Rotator) "180.000000,0.000000,0.000000" "0, 0, 0" _value_10) false false)
                    (Transformation|SetRelativeScale3D (Variables|Default|GetO) (Math|Vector|Lerp(Vector) "0, 0, 0" "1.000000,1.000000,1.000000" _value_10)))))
              (:then_3
                (Utilities|FlowControl|Delay 1.0)
                (bind _value_11 (Timeline|URotation PlayFromStart)
                  (:Update
                    (Transformation|SetRelativeRotation (Variables|Default|GetU) (Math|Rotator|Lerp(Rotator) "180.000000,0.000000,0.000000" "0, 0, 0" _value_11) false false)
                    (Transformation|SetRelativeScale3D (Variables|Default|GetU) (Math|Vector|Lerp(Vector) "0, 0, 0" "1.000000,1.000000,1.000000" _value_11)))))
              (:then_4
                (Utilities|FlowControl|Delay 1.12)
                (bind (_direction _value_12) (Timeline|PRotation PlayFromStart)
                  (:Update
                    (Transformation|SetRelativeRotation (Variables|Default|GetP) (Math|Rotator|Lerp(Rotator) "180.000000,0.000000,0.000000" "0, 0, 0" _value_12) false false)
                    (Transformation|SetRelativeScale3D (Variables|Default|GetP) (Math|Vector|Lerp(Vector) "0, 0, 0" "1.000000,1.000000,1.000000" _value_12))
                    (Rendering|Material|SetScalarParameterValueonMaterials (Variables|Default|GetBall) "VisibilityPercent" _value_12))
                  (:Finished
                    (switch Utilities|FlowControl|Switch|SwitchonETimelineDirection _direction
                      (:Forward
                        (CallFunction|Waiting))
                      (:Backward
                        (CallFunction|SetCommandsReceiving true)))))))))))))

(event Custom|Waiting
  (Utilities|FlowControl|Delay 1.4)
  (Utilities|FlowControl|Delay 2.2)
  (CallFunction|Disappearing))

(event Custom|Disappearing
  (Utilities|FlowControl|Sequence
    (:then_0
      (Utilities|FlowControl|Sequence
        (:then_0
          (Utilities|FlowControl|Delay 0.2)
          (bind _value (Timeline|SRotation ReverseFromEnd)
            (:Update
              (Transformation|SetRelativeRotation (Variables|Default|GetS) (Math|Rotator|Lerp(Rotator) "180.000000,0.000000,0.000000" "0, 0, 0" _value) false false)
              (Transformation|SetRelativeScale3D (Variables|Default|GetS) (Math|Vector|Lerp(Vector) "0, 0, 0" "1.000000,1.000000,1.000000" _value)))))
        (:then_1
          (Utilities|FlowControl|Delay 0.44)
          (bind _value_2 (Timeline|ERotation ReverseFromEnd)
            (:Update
              (Transformation|SetRelativeRotation (Variables|Default|GetE) (Math|Rotator|Lerp(Rotator) "180.000000,0.000000,0.000000" "0, 0, 0" _value_2) false false)
              (Transformation|SetRelativeScale3D (Variables|Default|GetE) (Math|Vector|Lerp(Vector) "0, 0, 0" "1.000000,1.000000,1.000000" _value_2)))))
        (:then_2
          (Utilities|FlowControl|Delay 0.56)
          (bind _value_3 (Timeline|NRotation ReverseFromEnd)
            (:Update
              (Transformation|SetRelativeRotation (Variables|Default|GetN) (Math|Rotator|Lerp(Rotator) "180.000000,0.000000,0.000000" "0, 0, 0" _value_3) false false)
              (Transformation|SetRelativeScale3D (Variables|Default|GetN) (Math|Vector|Lerp(Vector) "0, 0, 0" "1.000000,1.000000,1.000000" _value_3)))))
        (:then_3
          (Utilities|FlowControl|Delay 0.68)
          (bind _value_4 (Timeline|TRotation ReverseFromEnd)
            (:Update
              (Transformation|SetRelativeRotation (Variables|Default|GetT) (Math|Rotator|Lerp(Rotator) "180.000000,0.000000,0.000000" "0, 0, 0" _value_4) false false)
              (Transformation|SetRelativeScale3D (Variables|Default|GetT) (Math|Vector|Lerp(Vector) "0, 0, 0" "1.000000,1.000000,1.000000" _value_4)))))
        (:then_4
          (Utilities|FlowControl|Delay 0.8)
          (bind _value_5 (Timeline|R1Rotation ReverseFromEnd)
            (:Update
              (Transformation|SetRelativeRotation (Variables|Default|GetR1) (Math|Rotator|Lerp(Rotator) "180.000000,0.000000,0.000000" "0, 0, 0" _value_5) false false)
              (Transformation|SetRelativeScale3D (Variables|Default|GetR1) (Math|Vector|Lerp(Vector) "0, 0, 0" "1.000000,1.000000,1.000000" _value_5)))))))
    (:then_1
      (Utilities|FlowControl|Sequence
        (:then_0
          (Utilities|FlowControl|Delay 0.68)
          (bind _value_6 (Timeline|GRotation ReverseFromEnd)
            (:Update
              (Transformation|SetRelativeRotation (Variables|Default|GetG) (Math|Rotator|Lerp(Rotator) "180.000000,0.000000,0.000000" "0, 0, 0" _value_6) false false)
              (Transformation|SetRelativeScale3D (Variables|Default|GetG) (Math|Vector|Lerp(Vector) "0, 0, 0" "1.000000,1.000000,1.000000" _value_6)))))
        (:then_1
          (Utilities|FlowControl|Delay 0.84)
          (bind _value_7 (Timeline|R2Rotation ReverseFromEnd)
            (:Update
              (Transformation|SetRelativeRotation (Variables|Default|GetR2) (Math|Rotator|Lerp(Rotator) "180.000000,0.000000,0.000000" "0, 0, 0" _value_7) false false)
              (Transformation|SetRelativeScale3D (Variables|Default|GetR2) (Math|Vector|Lerp(Vector) "0, 0, 0" "1.000000,1.000000,1.000000" _value_7)))))
        (:then_2
          (Utilities|FlowControl|Delay 0.92)
          (bind _value_8 (Timeline|ORotation ReverseFromEnd)
            (:Update
              (Transformation|SetRelativeRotation (Variables|Default|GetO) (Math|Rotator|Lerp(Rotator) "180.000000,0.000000,0.000000" "0, 0, 0" _value_8) false false)
              (Transformation|SetRelativeScale3D (Variables|Default|GetO) (Math|Vector|Lerp(Vector) "0, 0, 0" "1.000000,1.000000,1.000000" _value_8)))))
        (:then_3
          (Utilities|FlowControl|Delay 1.0)
          (bind _value_9 (Timeline|URotation ReverseFromEnd)
            (:Update
              (Transformation|SetRelativeRotation (Variables|Default|GetU) (Math|Rotator|Lerp(Rotator) "180.000000,0.000000,0.000000" "0, 0, 0" _value_9) false false)
              (Transformation|SetRelativeScale3D (Variables|Default|GetU) (Math|Vector|Lerp(Vector) "0, 0, 0" "1.000000,1.000000,1.000000" _value_9)))))
        (:then_4
          (Utilities|FlowControl|Delay 1.12)
          (bind (_direction _value_10) (Timeline|PRotation ReverseFromEnd)
            (:Update
              (Transformation|SetRelativeRotation (Variables|Default|GetP) (Math|Rotator|Lerp(Rotator) "180.000000,0.000000,0.000000" "0, 0, 0" _value_10) false false)
              (Transformation|SetRelativeScale3D (Variables|Default|GetP) (Math|Vector|Lerp(Vector) "0, 0, 0" "1.000000,1.000000,1.000000" _value_10))
              (Rendering|Material|SetScalarParameterValueonMaterials (Variables|Default|GetBall) "VisibilityPercent" _value_10))
            (:Finished
              (switch Utilities|FlowControl|Switch|SwitchonETimelineDirection _direction
                (:Forward
                  (CallFunction|Waiting))
                (:Backward
                  (CallFunction|SetCommandsReceiving true))))))
        (:then_5
          (Utilities|FlowControl|Delay 1.12)
          (bind _value_11 (Timeline|BallDisappearing ReverseFromEnd)
            (:Update
              (Transformation|SetRelativeScale3D (Variables|Default|GetBall) (Math|Vector|Lerp(Vector) "0, 0, 0" "0.730000,0.730000,0.730000" _value_11)))))))))

(event EventBeginPlay
  (Rendering|SetActorHiddenInGame true))

(fn ConstructionScript)

(fn ResetState
  (Transformation|SetRelativeLocation (Variables|Default|GetBall) "0, 0, 0" false false)
  (Transformation|SetRelativeScale3D (Variables|Default|GetBall) "0, 0, 0")
  (Transformation|SetRelativeRotation (Variables|Default|GetS) "180.000000,0.000000,0.000000" false false)
  (Rendering|Material|SetScalarParameterValueonMaterials (Variables|Default|GetBall) "VisibilityPercent" 0.0))

(fn SetCommandsReceiving
  (params (Available :type Boolean))
  (if (!= Available (Variables|Properties|GetCommandsReceivingAvailable))
    (Variables|Properties|SetCommandsReceivingAvailable Available)))