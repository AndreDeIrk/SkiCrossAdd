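; Spline-following actor that moves its Plane component along a spline when the AnimatePlane event is called.
; A timeline drives two spline samples, spaced by the plane's length as a fraction of total spline length.
; The plane sits at their midpoint and faces from rear to front sample, combined with a timeline-driven roll, so its orientation follows the curve across its length.
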(event Custom|AnimatePlane
  (bind (_direction _value1 _rotation) (Timeline|Timeline PlayFromStart)
    (:Update
      (Transformation|SetRelativeLocationAndRotation (Variables|Default|GetPlane) (Math|Vector|Lerp(Vector) (Spline|GetLocationatTime (Variables|Default|GetSpline) (+ (* (Variables|Default|GetPlaneLengthScale) (/ 1e+02 (Spline|GetSplineLength (Variables|Default|GetSpline)))) _value1) "Local" false) (Spline|GetLocationatTime (Variables|Default|GetSpline) _value1 "Local" false) 0.5) (Math|Rotator|CombineRotators (Math|Rotator|MakeRotator _rotation 0.0 0.0) (Math|Rotator|FindLookatRotation (Spline|GetLocationatTime (Variables|Default|GetSpline) _value1 "Local" false) (Spline|GetLocationatTime (Variables|Default|GetSpline) (+ (* (Variables|Default|GetPlaneLengthScale) (/ 1e+02 (Spline|GetSplineLength (Variables|Default|GetSpline)))) _value1) "Local" false))) false false))))

(event Collision|EventActorBeginOverlap
  (params (OtherActor :type Actor%20Object%20Reference)))

(event EventTick
  (params (DeltaSeconds :type Float%20%28single-precision%29)))

(fn ConstructionScript)